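; BP_MHUD, apparently a HUD Blueprint, connects a possession widget to the game and refreshes its display.
; On BeginPlay it polls by function-name timer until PossessionWidget is valid, then casts it to WBP_Possessions and caches the reference.
; The UpdatePossessionUI event forwards to UpdatePossession on that cached widget, without a validity check.
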(event `self.ReceiveBeginPlay`
  (`parent.ReceiveBeginPlay`)
  (`self.Bind WBP Possession`))

(event `self.UpdatePossessionUI`
  (`/Game/_Game/UI/WBP_Possessions.UpdatePossession` (`self.As WBP Possessions`)))

(fn `Bind WBP Possession`
  (bind _possessionwidget (`self.PossessionWidget`))
  (`/Engine/EditorBlueprintResources/StandardMacros.IsValid` _possessionwidget
    (:`Is Valid`
      (bind _aswbp_possessions (cast `/Game/_Game/UI/WBP_Possessions` _possessionwidget))
      (set `self.As WBP Possessions` _aswbp_possessions))
    (:`Is Not Valid`
      (`KismetSystemLibrary.K2_SetTimer` null "Bind WBP Possession" 0.1))))

(fn `UserConstructionScript`)